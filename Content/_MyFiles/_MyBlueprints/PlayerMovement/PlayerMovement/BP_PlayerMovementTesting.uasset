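; Test player character Blueprint for movement, with tank-style controls, a crouch toggle and a flashlight toggle.
; BeginPlay adds the testing Enhanced Input mapping context to the player controller's subsystem and prints whether it succeeded.
; Move input drives only forward and backward along the actor's facing, while Turn input applies yaw rotation scaled by rotation rate and delta seconds.
; Boolean flags track crouch and flashlight state, with the light switched through its intensity.
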(event `EnhancedInput|/Game/_MyFiles/_MyBlueprints/PlayerMovement/PlayerInput/InputActions/IA_FlashlightToggle`
  (params (ActionValue :type Boolean) (ElapsedSeconds :type "Float (double-precision)") (TriggeredSeconds :type "Float (double-precision)") (InputAction :type "InputAction Object Reference" :default "/Game/_MyFiles/_MyBlueprints/PlayerMovement/PlayerInput/InputActions/IA_FlashlightToggle.IA_FlashlightToggle"))
  (bind _flashlightlight (`self.FlashlightLight`))
  ;[0.1382 0 0.15 0.5] Flashlight Toggle
  (:`Started`
    (if (`self.IsFlashlightOn`)
      (`LightComponent.SetIntensity` _flashlightlight 0.0)
      (set `self.IsFlashlightOn` false)
      (else
        (`LightComponent.SetIntensity` _flashlightlight (`self.FlashlightBrightness`))
        (set `self.IsFlashlightOn` true)))))

(event `EnhancedInput|/Game/_MyFiles/_MyBlueprints/PlayerMovement/PlayerInput/InputActions/IA_Crouch`
  (params (ActionValue :type Boolean) (ElapsedSeconds :type "Float (double-precision)") (TriggeredSeconds :type "Float (double-precision)") (InputAction :type "InputAction Object Reference" :default "/Game/_MyFiles/_MyBlueprints/PlayerMovement/PlayerInput/InputActions/IA_Crouch.IA_Crouch"))
  ;[0.15 0.1431 0 0.5 30] Player crouching
  (:`Started`
    (if (`self.IsPlayerCrouching`)
      (`self.UnCrouch`)
      (set `self.IsPlayerCrouching` false)
      (else
        (`self.Crouch`)
        (set `self.IsPlayerCrouching` true)))))

(event `EnhancedInput|/Game/_MyFiles/_MyBlueprints/PlayerMovement/PlayerInput/InputActions/IA_Turn`
  (params (ActionValue :type "Float (double-precision)") (ElapsedSeconds :type "Float (double-precision)") (TriggeredSeconds :type "Float (double-precision)") (InputAction :type "InputAction Object Reference" :default "/Game/_MyFiles/_MyBlueprints/PlayerMovement/PlayerInput/InputActions/IA_Turn.IA_Turn"))
  ;[0 1 0 0.5 30] Adding player rotation using input
  (:`Triggered`
    (`self.K2_AddActorWorldRotation` (* (* (`KismetMathLibrary.MakeRotator` 0.0 0.0 ActionValue) (`self.PlayerRotationRate`)) (stale `self.ReceiveTick` DeltaSeconds)))))

(event `self.ReceiveTick`
  (params (DeltaSeconds :type "Float (single-precision)"))
  ;[0 1 0 0.5 30] Adding player rotation using input
)

(event `EnhancedInput|/Game/_MyFiles/_MyBlueprints/PlayerMovement/PlayerInput/InputActions/IA_Move`
  (params (ActionValue :type "Vector2D Structure") (ElapsedSeconds :type "Float (double-precision)") (TriggeredSeconds :type "Float (double-precision)") (InputAction :type "InputAction Object Reference" :default "/Game/_MyFiles/_MyBlueprints/PlayerMovement/PlayerInput/InputActions/IA_Move.IA_Move"))
  ;[0 0.02589 0.15 0.5 30] Adding player movement input
  (:`Triggered`
    (`self.AddMovementInput` (`self.GetActorForwardVector`) ActionValue_Y)))

(event `self.ReceiveBeginPlay`
  ;[1 0 0.01066 0.5 30] Adding Mapping context
  (bind _asplayer_controller (cast `PlayerController` (`self.GetController`)))
  (bind _returnvalue (pcsubsystem `EnhancedInputLocalPlayerSubsystem` _asplayer_controller))
  (`/Engine/EditorBlueprintResources/StandardMacros.IsValid` _returnvalue
    (:`Is Valid`
      (`KismetSystemLibrary.PrintString` "Player Has IMC connected!" true true (struct :`G` 1.0 :`A` 1.0))
      (`EnhancedInputSubsystemInterface.AddMappingContext` _returnvalue "/Game/_MyFiles/_MyBlueprints/PlayerMovement/PlayerInput/IMC/IMC_TestingMovement.IMC_TestingMovement" 0 (struct)))
    (:`Is Not Valid`
      (`KismetSystemLibrary.PrintString` "ERROR: No mapping context for player" true true (struct :`R` 1.0 :`A` 1.0)))))

(fn `UserConstructionScript`)