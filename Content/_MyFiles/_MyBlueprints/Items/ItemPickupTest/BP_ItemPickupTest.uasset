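; A test item pickup actor that shows a prompt when the player comes within interaction range.
; On BeginPlay it sizes the PlayerDetection sphere from DetectionRadius and hides the UITest component.
; Overlap begin and end toggle UITest visibility, filtered by IsPlayerDetected to the first player character, and entering prints the item name.
; No actual pickup logic is implemented here.
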(event `self.ReceiveBeginPlay`
  (`SphereComponent.SetSphereRadius` (`self.PlayerDetection`) (`self.DetectionRadius`) true)
  (`SceneComponent.SetVisibility` (`self.UITest`) false false))

(event `self.PlayerDetection.OnComponentBeginOverlap`
  (params (OverlappedComponent :type "PrimitiveComponent Object Reference") (OtherActor :type "Actor Object Reference") (OtherComp :type "PrimitiveComponent Object Reference") (OtherBodyIndex :type Integer) (bFromSweep :type Boolean) (SweepResult :type "HitResult Structure (by ref)"))
  ; Entering interaction range
  (if (`self.IsPlayerDetected` OtherActor)
    (`SceneComponent.SetVisibility` (`self.UITest`) true false)
    (`KismetSystemLibrary.PrintString` (`KismetTextLibrary.Conv_TextToString` (`|FormatText` "Player found {Item Name}" (`self.ItemName`))))))

(event `self.PlayerDetection.OnComponentEndOverlap`
  (params (OverlappedComponent :type "PrimitiveComponent Object Reference") (OtherActor :type "Actor Object Reference") (OtherComp :type "PrimitiveComponent Object Reference") (OtherBodyIndex :type Integer))
  ; leaving interaction range
  (if (`self.IsPlayerDetected` OtherActor)
    (`SceneComponent.SetVisibility` (`self.UITest`) false false)))

(fn `IsPlayerDetected`
  (params (A :type "Object Object Reference"))
  (returns (`Return Value` :type Boolean))
  (return (== A (`GameplayStatics.GetPlayerCharacter` 0))))

(fn `UserConstructionScript`)